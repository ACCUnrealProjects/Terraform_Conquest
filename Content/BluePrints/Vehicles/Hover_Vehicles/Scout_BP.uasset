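; Scout hover vehicle pawn that manages its on-screen UI while a player controls it.
; On possession by a player controller, it creates a FloatingShipUI_BP widget, passes itself as the ShipActor, stores the widget and adds it to the viewport.
; On unpossession from a player controller, it removes that widget.
; The graphs shown hold no movement logic, and the construction script is empty.
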(event EventPossessed
  (params (NewController :type Controller%20Object%20Reference))
  (if (Class|Controller|IsPlayerController NewController)
    (bind _returnvalue (UserInterface|CreateWidget "/Game/HUD/FloatingShipUI_BP.FloatingShipUI_BP_C"))
    (Variables|/Game/HUD/FloatingShipUI_BP.FloatingShipUI_BP_C|SetShipActor _returnvalue self)
    (Variables|Default|SetHover_Veh_Widget _returnvalue)
    (UserInterface|Viewport|AddtoViewport _returnvalue 0)))

(event EventUnpossessed
  (params (OldController :type Controller%20Object%20Reference))
  (if (Class|Controller|IsPlayerController OldController)
    (Widget|RemovefromParent (Variables|Default|GetHover_Veh_Widget))))

(fn ConstructionScript)